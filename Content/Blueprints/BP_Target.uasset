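; BP_Target is a shootable target for a shooting range with a first-person game mode.
; The construction script copies HP into a working counter, which each Shot event lowers by one.
; At zero, Kill adds to the game mode's score, asks the ShootingRange to spawn another target, and destroys this actor.
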(event Custom|Shot
  (bind _output_get (Variables|Default|SetM_HP (- (Variables|Default|GetM_HP) 1)))
  (if (== _output_get 0)
    (CallFunction|Kill)))

(event EventBeginPlay)

(event Collision|EventActorBeginOverlap
  (params (OtherActor :type Actor%20Object%20Reference)))

(event EventTick
  (params (DeltaSeconds :type Float%20%28single-precision%29)))

(fn ConstructionScript
  (Variables|Default|SetM_HP (Variables|Default|GetHP)))

(fn Kill
  (bind _asbp_first_person_game_mode (Utilities|Casting|CastToBP_FirstPersonGameMode (Game|GetGameMode)))
  (Default|AddtoScore _asbp_first_person_game_mode)
  (Default|SpawnTarget (Variables|Default|GetShooting_Range))
  (Actor|DestroyActor))