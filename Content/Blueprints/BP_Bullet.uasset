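; BP_Bullet is a physics-driven projectile actor that destroys itself after a set lifetime.
; Fire clears the mesh's linear velocity, then applies a mass-dependent impulse along Direction scaled by Power.
; BeginPlay starts a timer by function name that calls Destroy after LifeTime.
; The file contains no hit or damage logic.
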(event EventBeginPlay
  (Utilities|Time|SetTimerbyFunctionName 0 "Destroy" (Variables|Default|GetLifeTime)))

(fn ConstructionScript)

(fn Fire
  (bind _power (Variables|Default|GetPower))
  (bind _mesh (Variables|Default|GetMesh))
  (Class|PrimitiveComponent|SetAllPhysicsLinearVelocity _mesh "0, 0, 0" false)
  (Physics|AddImpulse _mesh (* (Variables|Default|GetDirection) (Math|Vector|MakeVector _power _power _power)) "None" false))

(fn Destroy
  (Actor|DestroyActor))