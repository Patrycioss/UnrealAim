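; BP_TargetRack is a rack that spawns BP_Target actors for a shooting range.
; SpawnTarget picks a random point along M1's scaled local X bounds at its maximum Y edge, rotated into the component's orientation.
; Each target spawns yawed 90 degrees from M1 and receives the rack's ShootingRange reference.
; The event graph and construction script are empty, so spawning relies on external calls to SpawnTarget.
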(event EventBeginPlay)

(event Collision|EventActorBeginOverlap
  (params (OtherActor :type Actor%20Object%20Reference)))

(event EventTick
  (params (DeltaSeconds :type Float%20%28single-precision%29)))

(fn ConstructionScript)

(fn SpawnTarget
  (bind _m1 (Variables|Default|Getm1))
  (bind _returnvalue (Transformation|GetWorldScale _m1))
  (bind _returnvalue_2 (Transformation|GetWorldTransform _m1))
  (bind (_min _max) (Components|StaticMesh|GetLocalBounds _m1))
  (bind (_location _rotation) (Math|Transform|BreakTransform _returnvalue_2))
  (bind (_roll _pitch _yaw) (Math|Rotator|BreakRotator _rotation))
  (bind _output_get (LocalVariables|SetMinScaleld (* _min _returnvalue)))
  (bind _output_get_2 (LocalVariables|SetMaxScaled (* _max _returnvalue)))
  (bind _returnvalue_3 (Game|SpawnActorfromClass "/Game/Blueprints/BP_Target.BP_Target_C" (Math|Transform|MakeTransform (+ _location (Math|Vector|RotateVector (Math|Vector|MakeVector (Math|Random|RandomFloatinRange (.X (Class|KismetMathLibrary|BreakVector3f _output_get)) (.X (Class|KismetMathLibrary|BreakVector3f _output_get_2))) (.Y (Class|KismetMathLibrary|BreakVector3f _output_get_2)) 0.0) _rotation)) (Math|Rotator|MakeRotator _roll _pitch (+ _yaw 9e+01))) "Undefined" (Components|GetOwner _m1) 0))
  (Variables|/Game/Blueprints/BP_Target.BP_Target_C|SetShooting_Range _returnvalue_3 (Variables|Default|Getshooting_range)))