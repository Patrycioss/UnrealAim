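; BP_ShootingRange is a manager actor for a shooting range that spawns and clears targets.
; Its construction script gathers every BP_TargetRack in the level and gives each a reference back to itself.
; SpawnTarget asks a random rack to spawn a target, and Reset destroys all BP_Target actors.
; The event graph is inactive, so these functions depend on external callers.
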(event Input|EnhancedActionEvents|EnhancedInputActionIA_Test
  (params (ActionValue :type Boolean) (ElapsedSeconds :type Float%20%28double-precision%29) (TriggeredSeconds :type Float%20%28double-precision%29) (InputAction :type Input%20Action%20Object%20Reference :default "/Game/Input/IA_Test.IA_Test")))

(event EventBeginPlay)

(event Collision|EventActorBeginOverlap
  (params (OtherActor :type Actor%20Object%20Reference)))

(event EventTick
  (params (DeltaSeconds :type Float%20%28single-precision%29)))

(fn ConstructionScript
  (bind _outactors (Actor|GetAllActorsOfClass "/Game/Blueprints/BP_TargetRack.BP_TargetRack_C"))
  (bind _output_get (Variables|Default|SetTargetRacks _outactors))
  (for _array_element _output_get
    (Variables|/Game/Blueprints/BP_TargetRack.BP_TargetRack_C|Setshooting_range _array_element self)))

(fn SpawnTarget
  (Default|SpawnTarget (.OutItem (Utilities|Array|Random (Variables|Default|GetTargetRacks)))))

(fn Reset
  (bind _outactors (Actor|GetAllActorsOfClass "/Game/Blueprints/BP_Target.BP_Target_C"))
  (for _array_element _outactors
    (Actor|DestroyActor _array_element)))